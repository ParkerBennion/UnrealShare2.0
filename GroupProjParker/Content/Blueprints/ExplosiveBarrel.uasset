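; Explosive barrel actor that detonates when its capsule overlaps the player's hit box or a bullet.
; Detonation fires a radial force impulse and destroys the barrel.
; Player contact also deals damage and launches the character along a scaled vector pointing from the barrel's cylinder to player 0.
; A bullet hit destroys the bullet and detonates the barrel without directly hurting the player.
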(event OnComponentBeginOverlap(Capsule)
  (params (OverlappedComponent :type Primitive%20Component%20Object%20Reference) (OtherActor :type Actor%20Object%20Reference) (OtherComp :type Primitive%20Component%20Object%20Reference) (OtherBodyIndex :type Integer) (bFromSweep :type Boolean) (SweepResult :type Hit%20Result%20Structure%20%28by%20ref%29))
  (bind _radialforce (Variables|Default|GetRadialForce))
  (if (Components|ComponentHasTag OtherComp "PlayerHitBox")
    (bind _asfirst_person_character (Utilities|Casting|CastToFirstPersonCharacter OtherActor))
    (Class|RadialForceComponent|FireImpulse _radialforce)
    (Default|Hurt _asfirst_person_character 5e+01)
    (Character|LaunchCharacter _asfirst_person_character (* (- (.location (Transformation|GetActorTransform (Game|GetPlayerCharacter 0))) (Transformation|GetWorldLocation (Variables|Default|GetCylinder))) 15.0) false false)
    (else
      (bind _asbullet (Utilities|Casting|CastToBullet OtherActor))
      (Actor|DestroyActor _asbullet)
      (Class|RadialForceComponent|FireImpulse _radialforce)))
  (Actor|DestroyActor))

(fn ConstructionScript)