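; Game mode Blueprint that respawns the first-person player character whenever it is destroyed.
; On BeginPlay it binds to the player character's OnDestroyed event.
; After a brief delay, that event spawns a replacement at the stored SpawnLocation, adjusting for collisions, and has player controller 0 possess it.
; It then calls Respawn to rebind to the new pawn, so the cycle repeats on every death.
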(event Custom|OnDestroyed_Event
  (params (DestroyedActor :type Actor%20Object%20Reference))
  (Utilities|FlowControl|Delay 0.1)
  (bind _returnvalue (Game|SpawnActorfromClass "/Game/FirstPersonBP/Blueprints/FirstPersonCharacter.FirstPersonCharacter_C" (Variables|Default|GetSpawnLocation) "AdjustIfPossibleButAlwaysSpawn" 0 0))
  (Pawn|Possess (Game|GetPlayerController 0) _returnvalue)
  (CallFunction|Respawn))

(event Custom|Respawn
  (bind _asfirst_person_character (Utilities|Casting|CastToFirstPersonCharacter (Game|GetPlayerCharacter 0)))
  (Game|BindEventtoOnDestroyed _asfirst_person_character (delegate Custom|OnDestroyed_Event)))

(event EventBeginPlay
  (bind _asfirst_person_character (Utilities|Casting|CastToFirstPersonCharacter (Game|GetPlayerCharacter 0)))
  (Game|BindEventtoOnDestroyed _asfirst_person_character (delegate Custom|OnDestroyed_Event)))

(fn ConstructionScript)