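; FishCannon is a turret that fires homing fish at the player when it sees them.
; Its PawnSensing component filters sightings to BP_PlayerPawn, then a Delay holds back each shot and limits repeat firing.
; Each shot spawns a HomingFish at the FishSpawner transform and passes the player to its HomingProjectile function.
; The look-at rotation toward the player is disconnected, so this graph never turns the cannon.
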(event OnSeePawn(PawnSensing)
  (params (Pawn :type Pawn%20Object%20Reference))
  ;[1 1 1] Turret Homing
  (bind _asbp_player_pawn (Utilities|Casting|CastToBP_PlayerPawn Pawn))
  (Utilities|FlowControl|Sequence
    (:then_1
      (Utilities|FlowControl|Delay 3.0)
      (bind _returnvalue (Game|SpawnActorfromClass "/Game/MyBluePrints/HomingFish.HomingFish_C" (Transformation|GetWorldTransform (Variables|Default|GetFishSpawner)) "AdjustIfPossibleButAlwaysSpawn" 0 0))
      (Default|HomingProjectile _returnvalue _asbp_player_pawn))))

(fn ConstructionScript)