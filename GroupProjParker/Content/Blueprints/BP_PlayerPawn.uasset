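; BP_PlayerPawn is a rolling stone pawn, moved by torque, that pulls in, holds and blasts away nearby objects.
; Left Alt fires a suction impulse and sets SuctionOn, which makes Tick fire two holding impulses until Space blasts and activates particles.
; Both move axes share one torque node driving X and Y equally, while camera axes rotate the spring arm.
; K destroys the pawn and starts a camera fade.
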(event EventTick
  (params (DeltaSeconds :type Float%20%28single-precision%29))
  ;[1 1 1] Holds objects in a force field
  (if (Variables|Default|GetSuctionOn)
    (Utilities|FlowControl|Sequence
      (:then_0
        (Class|RadialForceComponent|FireImpulse (Variables|Default|GetForce)))
      (:then_1
        (Class|RadialForceComponent|FireImpulse (Variables|Default|GetInForce))))))

(event Input|AxisEvents|InputAxisMoveForwards/Backwards
  (params (AxisValue :type Float%20%28single-precision%29))
  ;[1 1 1] Move
  (Class|PrimitiveComponent|AddTorqueinRadians (Variables|Default|GetRollingStone) (Math|Vector|MakeVector (* (stale Input|AxisEvents|InputAxisMoveRight/Left AxisValue) (Variables|Default|GetTorqueStrength)) (* AxisValue (Variables|Default|GetTorqueStrength)) 0.0) "None" true))

(event Input|AxisEvents|InputAxisMoveRight/Left
  (params (AxisValue :type Float%20%28single-precision%29))
  ;[1 1 1] Move
  (Class|PrimitiveComponent|AddTorqueinRadians (Variables|Default|GetRollingStone) (Math|Vector|MakeVector (* AxisValue (Variables|Default|GetTorqueStrength)) (* (stale Input|AxisEvents|InputAxisMoveForwards/Backwards AxisValue) (Variables|Default|GetTorqueStrength)) 0.0) "None" true))

(event Input|AxisEvents|InputAxisCameraTurn
  (params (AxisValue :type Float%20%28single-precision%29))
  (Transformation|AddWorldRotation (Variables|Default|GetSpringArm) (Math|Rotator|MakeRotator 0.0 0.0 AxisValue) false false))

(event Input|AxisEvents|InputAxisCameraTilt
  (params (AxisValue :type Float%20%28single-precision%29))
  (Transformation|AddWorldRotation (Variables|Default|GetSpringArm) (Math|Rotator|MakeRotator 0.0 AxisValue 0.0) false false))

(event Input|KeyboardEvents|K
  (params (Key :type Key%20Structure :default "None"))
  ;[1 1 1] Kill Code
  (:Pressed
    (Actor|DestroyActor)
    (CameraFades|StartCameraFade :self (Game|GetPlayerCameraManager 0) :ToAlpha 1.0 :Duration 0.1)
    (Utilities|FlowControl|Delay 2.0)))

(event Input|KeyboardEvents|SpaceBar
  (params (Key :type Key%20Structure :default "None"))
  ;[1 1 1] Blows objects away
  (:Pressed
    (Variables|Default|SetSuctionOn false)
    (Utilities|FlowControl|Sequence
      (:then_0
        (Class|RadialForceComponent|FireImpulse (Variables|Default|GetBlastForce))
        (Development|PrintString "Boom"))
      (:then_1
        (Components|Activation|Activate (Variables|Default|GetParticleSystem) false)))))

(event Input|KeyboardEvents|LeftAlt
  (params (Key :type Key%20Structure :default "None"))
  ;[1 1 1] Sucks in nearby objects
  (:Pressed
    (Variables|Default|SetSuctionOn true)
    (Class|RadialForceComponent|FireImpulse (Variables|Default|GetSuckforce))))

(fn ConstructionScript)