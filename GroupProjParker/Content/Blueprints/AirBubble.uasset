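; AirBubble is a moving gravity-volume actor that applies a force to the player's roller while the player is inside it.
; Collider overlaps toggle a flag that gates Tick, which adds a linear-falloff radial acceleration to the BP_PlayerPawn's Roller, centered at an offset from the player's location.
; The construction script configures InterpToMovement with two relative control points and a duration, both driven by variables.
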(event OnComponentBeginOverlap(colider)
  (params (OverlappedComponent :type Primitive%20Component%20Object%20Reference) (OtherActor :type Actor%20Object%20Reference) (OtherComp :type Primitive%20Component%20Object%20Reference) (OtherBodyIndex :type Integer) (bFromSweep :type Boolean) (SweepResult :type Hit%20Result%20Structure%20%28by%20ref%29))
  ;[1 1 1] Gravity Volume
  (Variables|Default|SetBool true))

(event OnComponentEndOverlap(colider)
  (params (OverlappedComponent :type Primitive%20Component%20Object%20Reference) (OtherActor :type Actor%20Object%20Reference) (OtherComp :type Primitive%20Component%20Object%20Reference) (OtherBodyIndex :type Integer))
  ;[1 1 1] Gravity Volume
  (Utilities|Casting|CastToBP_PlayerPawn OtherActor)
  (Variables|Default|SetBool false))

(event EventTick
  (params (DeltaSeconds :type Float%20%28single-precision%29))
  ;[1 1 1] Gravity Volume
  (if (Variables|Default|GetBool)
    (bind _asbp_player_pawn (Utilities|Casting|CastToBP_PlayerPawn (stale OnComponentBeginOverlap(colider) OtherActor)))
    (Physics|AddRadialForce (Variables|/Game/MyBluePrints/BP_PlayerPawn.BP_PlayerPawn_C|GetRoller _asbp_player_pawn) (+ (Transformation|GetActorLocation (Game|Player|GetPlayerPawn 0)) (Variables|Default|GetAbovePlayer)) 4e+02 (Variables|Default|GetStrength) "RIF_Linear" true)))

(fn ConstructionScript
  (bind _interptomovement (Variables|Default|GetInterpToMovement))
  (Variables|/Script/Engine.InterpToMovementComponent|SetControlPoints _interptomovement (Utilities|Array|MakeArray (Utilities|Struct|MakeInterpControlPoint (Variables|Default|GetNewVar_0) true) (Utilities|Struct|MakeInterpControlPoint (Variables|Default|GetNewVar_1) true)))
  (Variables|/Script/Engine.InterpToMovementComponent|SetDuration _interptomovement (Variables|Default|Getduration)))