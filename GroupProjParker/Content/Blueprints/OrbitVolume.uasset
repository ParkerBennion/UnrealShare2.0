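; OrbitVolume is a gravity volume that applies a radial force to the player pawn's Roller around its Sphere.
; While the Colider overlap flag is set, Tick applies mass-independent force with linear falloff and zeroes the pawn's ForceStrength once.
; Exiting clears the flag, restores ForceStrength and resets the DoOnce.
; Player overlap with ButtonCollider sets Strength outward, then strongly inward after a short delay.
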(event OnComponentBeginOverlap(ButtonCollider)
  (params (OverlappedComponent :type Primitive%20Component%20Object%20Reference) (OtherActor :type Actor%20Object%20Reference) (OtherComp :type Primitive%20Component%20Object%20Reference) (OtherBodyIndex :type Integer) (bFromSweep :type Boolean) (SweepResult :type Hit%20Result%20Structure%20%28by%20ref%29))
  ;[1 1 1] Gravity Volume
  (Utilities|Casting|CastToBP_PlayerPawn OtherActor)
  (Variables|Default|SetStrength 1.5e+03)
  (Utilities|FlowControl|Delay 1.5)
  (Variables|Default|SetStrength -3e+04))

(event OnComponentBeginOverlap(colider)
  (params (OverlappedComponent :type Primitive%20Component%20Object%20Reference) (OtherActor :type Actor%20Object%20Reference) (OtherComp :type Primitive%20Component%20Object%20Reference) (OtherBodyIndex :type Integer) (bFromSweep :type Boolean) (SweepResult :type Hit%20Result%20Structure%20%28by%20ref%29))
  ;[1 1 1] Gravity Volume
  (Variables|Default|SetBool true))

(event OnComponentEndOverlap(colider)
  (params (OverlappedComponent :type Primitive%20Component%20Object%20Reference) (OtherActor :type Actor%20Object%20Reference) (OtherComp :type Primitive%20Component%20Object%20Reference) (OtherBodyIndex :type Integer))
  ;[1 1 1] Gravity Volume
  (Utilities|Casting|CastToBP_PlayerPawn OtherActor)
  (Variables|Default|SetBool false)
  (Variables|/Game/MyBluePrints/BP_PlayerPawn.BP_PlayerPawn_C|SetForceStrength (stale EventTick _asbp_player_pawn) 1e+01)
  (Utilities|FlowControl|DoOnce false) ; enters at Reset
)

(event EventTick
  (params (DeltaSeconds :type Float%20%28single-precision%29))
  ;[1 1 1] Gravity Volume
  (if (Variables|Default|GetBool)
    (bind _asbp_player_pawn (Utilities|Casting|CastToBP_PlayerPawn (stale OnComponentBeginOverlap(colider) OtherActor)))
    (Physics|AddRadialForce (Variables|/Game/MyBluePrints/BP_PlayerPawn.BP_PlayerPawn_C|GetRoller _asbp_player_pawn) (Transformation|GetWorldLocation (Variables|Default|GetSphere)) 4e+03 (Variables|Default|GetStrength) "RIF_Linear" true)
    (Utilities|FlowControl|DoOnce false
      (:Completed
        (Variables|/Game/MyBluePrints/BP_PlayerPawn.BP_PlayerPawn_C|SetForceStrength _asbp_player_pawn 0.0)
        (Development|PrintString "thrustnull")))))

(fn ConstructionScript)