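; WallPull1 is a gravity volume that pulls the player's roller toward a point offset from the pawn by AbovePlayer.
; Box or sphere overlaps toggle a flag that gates Tick, which applies a constant-falloff, negative-strength radial force as an acceleration change.
; Each active tick also moves KaiPlanet to that force origin.
; Roller gravity stays enabled, since both overlap begin and end set GravBool true.
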(event OnComponentBeginOverlap(SphereColider)
  (params (OverlappedComponent :type Primitive%20Component%20Object%20Reference) (OtherActor :type Actor%20Object%20Reference) (OtherComp :type Primitive%20Component%20Object%20Reference) (OtherBodyIndex :type Integer) (bFromSweep :type Boolean) (SweepResult :type Hit%20Result%20Structure%20%28by%20ref%29))
  ;[1 1 1] Gravity Volume
  (Variables|Default|SetBool true)
  (Variables|Default|SetGravBool true))

(event OnComponentEndOverlap(SphereColider)
  (params (OverlappedComponent :type Primitive%20Component%20Object%20Reference) (OtherActor :type Actor%20Object%20Reference) (OtherComp :type Primitive%20Component%20Object%20Reference) (OtherBodyIndex :type Integer))
  ;[1 1 1] Gravity Volume
  (Utilities|Casting|CastToBP_PlayerPawn (stale OnComponentEndOverlap(Box) OtherActor))
  (Variables|Default|SetBool false)
  (Variables|Default|SetGravBool true)
  (Physics|SetEnableGravity (Variables|/Game/MyBluePrints/BP_PlayerPawn.BP_PlayerPawn_C|GetRoller (stale EventTick _asbp_player_pawn)) (Variables|Default|GetGravBool)))

(event OnComponentBeginOverlap(Box)
  (params (OverlappedComponent :type Primitive%20Component%20Object%20Reference) (OtherActor :type Actor%20Object%20Reference) (OtherComp :type Primitive%20Component%20Object%20Reference) (OtherBodyIndex :type Integer) (bFromSweep :type Boolean) (SweepResult :type Hit%20Result%20Structure%20%28by%20ref%29))
  ;[1 1 1] Gravity Volume
  (Variables|Default|SetBool true)
  (Variables|Default|SetGravBool true))

(event OnComponentEndOverlap(Box)
  (params (OverlappedComponent :type Primitive%20Component%20Object%20Reference) (OtherActor :type Actor%20Object%20Reference) (OtherComp :type Primitive%20Component%20Object%20Reference) (OtherBodyIndex :type Integer))
  ;[1 1 1] Gravity Volume
  (Utilities|Casting|CastToBP_PlayerPawn OtherActor)
  (Variables|Default|SetBool false)
  (Variables|Default|SetGravBool true)
  (Physics|SetEnableGravity (Variables|/Game/MyBluePrints/BP_PlayerPawn.BP_PlayerPawn_C|GetRoller (stale EventTick _asbp_player_pawn)) (Variables|Default|GetGravBool)))

(event EventTick
  (params (DeltaSeconds :type Float%20%28single-precision%29))
  (bind _returnvalue (Game|Player|GetPlayerPawn 0))
  (bind _aboveplayer (Variables|Default|GetAbovePlayer))
  (bind _returnvalue_2 (Transformation|GetActorLocation _returnvalue))
  (bind _returnvalue_3 (+ _returnvalue_2 _aboveplayer))
  ;[1 1 1] Gravity Volume
  (if (Variables|Default|GetBool)
    (bind _asbp_player_pawn (Utilities|Casting|CastToBP_PlayerPawn (stale OnComponentBeginOverlap(Box) OtherActor)))
    (Physics|AddRadialForce (Variables|/Game/MyBluePrints/BP_PlayerPawn.BP_PlayerPawn_C|GetRoller _asbp_player_pawn) _returnvalue_3 4e+03 -6.8e+02 "RIF_Constant" true)
    (Transformation|SetWorldTransform (Variables|Default|GetKaiPlanet) (Math|Conversions|ToTransform(Vector) _returnvalue_3) false false)
    (Physics|SetEnableGravity (Variables|/Game/MyBluePrints/BP_PlayerPawn.BP_PlayerPawn_C|GetRoller _asbp_player_pawn) (Variables|Default|GetGravBool))))

(fn ConstructionScript)